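; BP_GoodCube is the correct physics cube of a puzzle (Enigme1) that opens a door when placed on a slot.
; On BeginPlay it enables physics on its cube and caches the level's BP_Door.
; When its box overlaps a BP_Slot, it activates the door's InterpToMovement, fires the door's CustomEvent and turns the slot's cube green.
; Leftover debug prints remain.
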(event OnComponentBeginOverlap(Box)
  (params (OverlappedComponent :type Primitive%20Component%20Object%20Reference) (OtherActor :type Actor%20Object%20Reference) (OtherComp :type Primitive%20Component%20Object%20Reference) (OtherBodyIndex :type Integer) (bFromSweep :type Boolean) (SweepResult :type Hit%20Result%20Structure%20%28by%20ref%29))
  (bind _asbp_slot (Utilities|Casting|CastToBP_Slot OtherActor))
  (Development|PrintString "coucouu")
  (CallFunction|OpenDoor)
  (Rendering|Material|SetMaterial (Variables|/Game/Enigme1/BP_Slot.BP_Slot_C|GetCube _asbp_slot) 0 "/Game/Enigme1/FakeLeVert.FakeLeVert"))

(event EventBeginPlay
  (Physics|SetSimulatePhysics (Variables|Default|GetCube) true)
  (bind _returnvalue (Actor|GetActorOfClass "/Game/Enigme1/BP_Door.BP_Door_C"))
  (Variables|Default|SetDoorRef _returnvalue))

(event Collision|EventActorBeginOverlap
  (params (OtherActor :type Actor%20Object%20Reference)))

(event EventTick
  (params (DeltaSeconds :type Float%20%28single-precision%29)))

(fn ConstructionScript)

(fn OpenDoor
  (bind _doorref (Variables|Default|GetDoorRef))
  (Development|PrintString "oprn")
  (Components|Activation|Activate (Variables|/Game/Enigme1/BP_Door.BP_Door_C|GetInterpToMovement _doorref) false)
  (Default|CustomEvent _doorref)
  (return))