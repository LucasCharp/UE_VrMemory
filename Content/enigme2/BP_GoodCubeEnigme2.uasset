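; Physics cube for puzzle 2 ("enigme2") that counts toward a referenced door when placed in a free BP_Slot2.
; Activation toggles the cube's active flag, swapping red and blue materials and printing the state.
; When its box overlaps a free slot while active, it deactivates, calls AddMessage on the door, stops simulating physics, and marks the slot taken with a green-named material.
; End overlap is empty; the LessMessage removal logic is disconnected.
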(event OnComponentBeginOverlap(Box)
  (params (OverlappedComponent :type Primitive%20Component%20Object%20Reference) (OtherActor :type Actor%20Object%20Reference) (OtherComp :type Primitive%20Component%20Object%20Reference) (OtherBodyIndex :type Integer) (bFromSweep :type Boolean) (SweepResult :type Hit%20Result%20Structure%20%28by%20ref%29))
  (bind _asbp_slot_2 (Utilities|Casting|CastToBP_Slot2 OtherActor))
  (if (not (Variables|/Game/enigme2/BP_Slot2.BP_Slot2_C|GetiamTake _asbp_slot_2))
    (if (Variables|Default|Getactivate)
      (Variables|Default|Setactivate false)
      (Class|BPIAdd|Add(Message) (Variables|Default|Getdoorref))
      (Physics|SetSimulatePhysics (Variables|Default|GetCube) false)
      (Variables|/Game/enigme2/BP_Slot2.BP_Slot2_C|SetiamTake _asbp_slot_2 true)
      (Rendering|Material|SetMaterial (Variables|/Game/enigme2/BP_Slot2.BP_Slot2_C|GetCube _asbp_slot_2) 0 "/Game/Enigme1/FakeLeVert.FakeLeVert"))))

(event OnComponentEndOverlap(Box)
  (params (OverlappedComponent :type Primitive%20Component%20Object%20Reference) (OtherActor :type Actor%20Object%20Reference) (OtherComp :type Primitive%20Component%20Object%20Reference) (OtherBodyIndex :type Integer)))

(event EventBeginPlay
  (Physics|SetSimulatePhysics (Variables|Default|GetCube) true))

(event Collision|EventActorBeginOverlap
  (params (OtherActor :type Actor%20Object%20Reference)))

(event EventTick
  (params (DeltaSeconds :type Float%20%28single-precision%29)))

(fn ConstructionScript)

(fn Activation
  (if (Variables|Default|Getactivate)
    (Variables|Default|Setactivate false)
    (Rendering|Material|SetMaterial (Variables|Default|GetCube) 0 "/Game/enigme2/M_LeRouge.M_LeRouge")
    (Development|PrintString "desactivate")
    (else
      (Variables|Default|Setactivate true)
      (Rendering|Material|SetMaterial (Variables|Default|GetCube) 0 "/Game/enigme2/M_LeBleu.M_LeBleu")
      (Development|PrintString "activate")))
  (return))