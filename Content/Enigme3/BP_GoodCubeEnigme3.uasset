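; BP_GoodCubeEnigme3 is a physics-simulated puzzle cube for Enigme 3 that counts toward a door when placed in a slot.
; Activation toggles its active state, swapping between red and blue materials.
; When its Box overlaps a free BP_Slot3 while active, it calls AddMessage on Doorref, stops simulating physics, claims the slot and turns it emissive green.
; End overlap does nothing, and the LessMessage branch never runs.
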(event OnComponentBeginOverlap(Box)
  (params (OverlappedComponent :type Primitive%20Component%20Object%20Reference) (OtherActor :type Actor%20Object%20Reference) (OtherComp :type Primitive%20Component%20Object%20Reference) (OtherBodyIndex :type Integer) (bFromSweep :type Boolean) (SweepResult :type Hit%20Result%20Structure%20%28by%20ref%29))
  (bind _asbp_slot_3 (Utilities|Casting|CastToBP_Slot3 OtherActor))
  (if (not (Variables|/Game/Enigme3/BP_Slot3.BP_Slot3_C|GetiamTake _asbp_slot_3))
    (if (Variables|Default|Getactivate)
      (Class|BPIAdd|Add(Message) (Variables|Default|Getdoorref))
      (Physics|SetSimulatePhysics (Variables|Default|GetCube) false)
      (Variables|/Game/Enigme3/BP_Slot3.BP_Slot3_C|SetiamTake _asbp_slot_3 true)
      (Rendering|Material|SetMaterial (Variables|/Game/Enigme3/BP_Slot3.BP_Slot3_C|GetCube _asbp_slot_3) 0 "/Game/AssetsDoor/emissive_green.emissive_green"))))

(event OnComponentEndOverlap(Box)
  (params (OverlappedComponent :type Primitive%20Component%20Object%20Reference) (OtherActor :type Actor%20Object%20Reference) (OtherComp :type Primitive%20Component%20Object%20Reference) (OtherBodyIndex :type Integer)))

(event EventBeginPlay
  (Physics|SetSimulatePhysics (Variables|Default|GetCube) true))

(event Collision|EventActorBeginOverlap
  (params (OtherActor :type Actor%20Object%20Reference)))

(event EventTick
  (params (DeltaSeconds :type Float%20%28single-precision%29)))

(fn ConstructionScript)

(fn Activation
  (if (Variables|Default|Getactivate)
    (Variables|Default|Setactivate false)
    (Rendering|Material|SetMaterial (Variables|Default|GetCube) 0 "/Game/enigme2/M_LeRouge.M_LeRouge")
    (Development|PrintString "desactivate")
    (else
      (Variables|Default|Setactivate true)
      (Rendering|Material|SetMaterial (Variables|Default|GetCube) 0 "/Game/enigme2/M_LeBleu.M_LeBleu")
      (Development|PrintString "activate")))
  (return))