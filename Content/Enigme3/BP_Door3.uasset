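; BP_Door3 is a puzzle door in Enigme3 that opens once its counter reaches two.
; The Add and Less events pass +1 or -1 to Check, which updates Count and prints debug messages.
; At the threshold, Check activates the InterpToMovement component, then CustomEvent destroys the Target and Target0 actors after a three-second delay.
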(event Custom|CustomEvent
  (Utilities|FlowControl|Delay 3.0)
  (Actor|DestroyActor (Variables|Default|GetTarget))
  (Actor|DestroyActor (Variables|Default|GetTarget_0)))

(event EventBeginPlay)

(event Collision|EventActorBeginOverlap
  (params (OtherActor :type Actor%20Object%20Reference)))

(event EventTick
  (params (DeltaSeconds :type Float%20%28single-precision%29)))

(event EventLess
  (CallFunction|Check -1))

(event EventAdd
  (CallFunction|Check 1))

(fn ConstructionScript)

(fn Check
  (params (Delta :type Integer))
  (Development|PrintString "Hello")
  (Variables|Default|SetCount (+ (Variables|Default|GetCount) Delta))
  (if (>= (Variables|Default|GetCount) 2)
    (Development|PrintString "Open")
    (Components|Activation|Activate (Variables|Default|GetInterpToMovement) false)
    (CallFunction|CustomEvent)
    (else
      (Development|PrintString "notopenyet"))))